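; Area-of-interest trigger actor that halts the top-down character and logs an event when entered.
; While active, an ActionBox overlap stores the character as interactable and zeroes its max walk speed.
; It also sends its message and itself to the game mode's EventLogComponent, even if the overlapping actor isn't a TopDownCharacter.
; Deactivate clears the active flag and switches the marker cube to a green translucent material; it does not restore walk speed.
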(event OnComponentBeginOverlap(ActionBox)
  (params (OverlappedComponent :type Primitive%20Component%20Object%20Reference) (OtherActor :type Actor%20Object%20Reference) (OtherComp :type Primitive%20Component%20Object%20Reference) (OtherBodyIndex :type Integer) (bFromSweep :type Boolean) (SweepResult :type Hit%20Result%20Structure%20%28by%20ref%29))
  (if (Variables|Default|GetIsActive)
    (CallFunction|SetInteractableCharacter OtherActor)
    (CallFunction|AddEventLog)))

(event EventBeginPlay)

(event Collision|EventActorBeginOverlap
  (params (OtherActor :type Actor%20Object%20Reference)))

(event EventTick
  (params (DeltaSeconds :type Float%20%28single-precision%29)))

(fn ConstructionScript)

(fn AddEventLog
  (bind _astop_down_game_mode (Utilities|Casting|CastToTopDownGameMode (Game|GetGameMode)))
  (Default|AddEvent (Variables|/Game/TopDownBP/Blueprints/TopDownGameMode.TopDownGameMode_C|GetEventLog_component _astop_down_game_mode) (Variables|Default|Getmsg) self))

(fn SetInteractableCharacter
  (params (Object :type Object%20Object%20Reference))
  (bind _astop_down_character (Utilities|Casting|CastToTopDownCharacter Object))
  (Variables|Default|SetinteractableCharacter _astop_down_character)
  (Variables|/Script/Engine.CharacterMovementComponent|SetMaxWalkSpeed (Variables|/Script/Engine.Character|GetCharacterMovement _astop_down_character) 0.0))

(fn Deactivate
  (Variables|Default|SetIsActive false)
  (Rendering|Material|SetMaterial (Variables|Default|GetAreaMarkerCube) 0 "/Game/HUD/M_GreenTrans.M_GreenTrans"))