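; BP_OpenLevelInteract is an interactable, door-style actor that sends the player to another level.
; On its first OnInteract from the character, guarded by a DoOnce with no reset, it optionally unlocks a level by index when the UnlockLevel flag is set.
; It then messages the game instance to join the named level, passing the DoorPosition world transform as the new position.
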(event EventBeginPlay
  (|CallParentFunction) ; This node is disabled and will not be called.\nDrag off pins to build functionality.
)

(event EventOnInteract
  ;[1 1 1] Override OnInteract and called from Character
  (Utilities|FlowControl|DoOnce false
    (:Completed
      (if (not (Variables|Setting|UnlockLevel|GetUnlockLevel?))
        _
        (else
          (CallFunction|UnlockLevel (Variables|Setting|UnlockLevel|GetLevelIndex) true)))
      (Class|BPMainMenuInterface|MSGJoinLevel(Message) (Game|GetGameInstance) (Variables|Setting|GetLevelName) 0 (Transformation|GetWorldTransform (Variables|Default|GetDoorPosition))))))

(fn ConstructionScript
  (|CallParentFunction))